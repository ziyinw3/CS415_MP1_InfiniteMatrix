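; BP_Tunnel is an endless-tunnel segment with a rotating holed wall that damages the player and destroys projectiles on overlap.
; Its trigger zone has TunnelSpawner spawn the next segment, removes this one, and scores the player unless the wall flagged a hit.
; Helper functions, not called within this Blueprint, randomize the wall's mesh and roll and spawn a health pack and an enemy on independent coin flips, keeping references to both.
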(event OnComponentBeginOverlap(TriggerZone)
  (params (OverlappedComponent :type Primitive%20Component%20Object%20Reference) (OtherActor :type Actor%20Object%20Reference) (OtherComp :type Primitive%20Component%20Object%20Reference) (OtherBodyIndex :type Integer) (bFromSweep :type Boolean) (SweepResult :type Hit%20Result%20Structure%20%28by%20ref%29))
  (Utilities|FlowControl|Sequence
    (:then_0
      (bind _asbp_player (Utilities|Casting|CastToBP_Player OtherActor))
      (Utilities|FlowControl|Sequence
        (:then_0
          (Default|SpawnTunnelatSpawnPoint (Variables|Default|GetTunnelSpawner))
          (CallFunction|DestroyEntities)
          (Actor|DestroyActor))
        (:then_1
          (if (Variables|/Game/InfiniteMatrix/Blueprints/BP_Player.BP_Player_C|GetHitWall _asbp_player)
            (Variables|/Game/InfiniteMatrix/Blueprints/BP_Player.BP_Player_C|SetHitWall _asbp_player false)
            (else
              (bind _result (Math|Integer|IncrementInt (Variables|/Game/InfiniteMatrix/Blueprints/BP_Player.BP_Player_C|GetScore _asbp_player))
                (:%20%20
                  (Variables|/Game/InfiniteMatrix/Blueprints/BP_Player.BP_Player_C|SetScore _asbp_player _result))))))))))

(event OnComponentBeginOverlap(WallMesh)
  (params (OverlappedComponent :type Primitive%20Component%20Object%20Reference) (OtherActor :type Actor%20Object%20Reference) (OtherComp :type Primitive%20Component%20Object%20Reference) (OtherBodyIndex :type Integer) (bFromSweep :type Boolean) (SweepResult :type Hit%20Result%20Structure%20%28by%20ref%29))
  (Utilities|FlowControl|Sequence
    (:then_0
      (bind _asbp_player (Utilities|Casting|CastToBP_Player OtherActor))
      (Utilities|FlowControl|Sequence
        (:then_0
          (Game|Damage|ApplyDamage _asbp_player 1e+01 0 0))
        (:then_1
          (Variables|/Game/InfiniteMatrix/Blueprints/BP_Player.BP_Player_C|SetHitWall _asbp_player true))))
    (:then_1
      (bind _asbp_projectile (Utilities|Casting|CastToBP_Projectile OtherActor))
      (Audio|PlaySound2D "/Game/InfiniteMatrix/Audio/wall_hit.wall_hit" 1.0 1.0 0.0 0 0)
      (Actor|DestroyActor _asbp_projectile))))

(event EventBeginPlay)

(event EventTick
  (params (DeltaSeconds :type Float%20%28single-precision%29))
  (Utilities|FlowControl|Sequence
    (:then_0
      (Transformation|AddLocalRotation (Variables|Default|GetWallMesh) (Math|Rotator|MakeRotator (* DeltaSeconds (Variables|Default|GetRotateSpeed)) 0.0 0.0) false false))))

(fn ConstructionScript)

(fn RandomizeWall
  (Components|StaticMesh|SetStaticMesh (Variables|Default|GetWallMesh) (Utilities|Select :Index (Math|Random|RandomIntegerinRange 0 3) :Option%200 "/Game/InfiniteMatrix/Meshes/SM_Hole_01.SM_Hole_01" :Option%201 "/Game/InfiniteMatrix/Meshes/SM_Hole_02.SM_Hole_02" :Option%202 "/Game/InfiniteMatrix/Meshes/SM_Hole_03.SM_Hole_03" :Option%203 "/Game/InfiniteMatrix/Meshes/SM_Hole_04.SM_Hole_04"))
  (Transformation|AddLocalRotation (Variables|Default|GetWallMesh) (Math|Rotator|MakeRotator (Math|Random|RandomFloatinRange 0.0 3.6e+02) 0.0 0.0) false false))

(fn SpawnEntities
  (Utilities|FlowControl|Sequence
    (:then_0
      (if (!= (Math|Random|RandomIntegerinRange 0 1) 0)
        (CallFunction|SpawnHealthPack)))
    (:then_1
      (if (== (Math|Random|RandomIntegerinRange 0 1) 0)
        (CallFunction|SpawnEnemy)))))

(fn SpawnHealthPack
  (bind _returnvalue (Game|SpawnActorfromClass "/Game/InfiniteMatrix/Blueprints/BP_Healthpack.BP_Healthpack_C" (Math|Transform|MakeTransform (+ (Transformation|GetWorldLocation (Variables|Default|GetCenter)) (Math|Vector|MakeVector (Math|Random|RandomFloatinRange -1e+02 1e+02) (Math|Random|RandomFloatinRange -3e+02 3e+02) (Math|Random|RandomFloatinRange -3e+02 3e+02))) (Math|Rotator|MakeRotator (Math|Random|RandomFloatinRange -2e+01 2e+01) 0.0 (Math|Random|RandomFloatinRange -3e+01 3e+01)) "1.000000,1.000000,1.000000") "Undefined" "MultiplyWithRoot" 0 0))
  (Variables|Default|SetHealthpack_Ref _returnvalue))

(fn DestroyEntities
  (Utilities|FlowControl|Sequence
    (:then_0
      (if (Utilities|IsValid (Variables|Default|GetHealthpack_Ref))
        (Actor|DestroyActor)))
    (:then_1
      (if (Utilities|IsValid (Variables|Default|GetEnemyRef))
        (Actor|DestroyActor)))))

(fn SpawnEnemy
  (bind _returnvalue (Math|Random|RandomFloatinRange 0.0 3.6e+02))
  (bind _returnvalue_2 (Math|Random|RandomFloatinRange 8e+02 1e+03))
  (bind _returnvalue_3 (Game|SpawnActorfromClass "/Game/InfiniteMatrix/Blueprints/BP_Enemy.BP_Enemy_C" (Math|Transform|MakeTransform (+ (Transformation|GetWorldLocation (Variables|Default|GetSpawnPoint)) (Math|Vector|MakeVector 0.0 (* (Math|Trig|Sin(Degrees) _returnvalue) _returnvalue_2) (* (Math|Trig|Cos(Degrees) _returnvalue) _returnvalue_2))) (Math|Rotator|MakeRotator 0.0 0.0 0.0) "1.000000,1.000000,1.000000") "Undefined" "MultiplyWithRoot" 0 0))
  (Variables|Default|SetEnemyRef _returnvalue_3))